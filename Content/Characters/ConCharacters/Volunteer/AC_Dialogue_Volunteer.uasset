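; Dialogue component for the convention Volunteer NPC, who gives the player clues about a lost keychain, a rude mother and son, and the recent death.
; It overrides Dialogue, calls the parent, resets DialogueIndex and switches on DialogueTreeIndex, with only tree 0 defined.
; Chained AddDialogue calls branch on the chosen option, each ending in CloseConversation after one reply.
; A fourth "How can i help" branch has no matching option in the opening prompt.
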(fn `Dialogue`
  (`parent.Dialogue`)
  (set `self.DialogueIndex` -1)
  (switch `int` (`self.DialogueTreeIndex`)
    (:`0`
      (bind (_state _optionindex) (`self.AddDialogue` "Volunteer" "Can I help you?" (`|MakeArray` "Did you find any lost keychains last night?" "I heard that lady over there gave you an earful yesterday." "Surprised to see the con still happening given what occurred last night." :!type "Text")))
      (switch `/Game/Blueprint/Enum_DiaState` _state
        (:`NewEnumerator0`
          (switch `int` _optionindex
            (:`0`
              (bind (_state_2 _optionindex_2) (`self.AddDialogue` "Volunteer" "Yeah actually, this really enthusiastic girl accidentally bumped into another volunteer and dropped a bunch all over the floor. He helped best he could from what I saw but one got missed. I stuck it in the lost and found box by the entrance. I would have helped but I was busy getting chewed out by this entitled lady and her kid" (`|MakeArray` "Sorry. Yesterday must have been brutal" :!type "Text")))
              (switch `/Game/Blueprint/Enum_DiaState` _state_2
                (:`NewEnumerator0`
                  (switch `int` _optionindex_2
                    (:`0`
                      (`self.CloseConversation` :!label _label))))))
            (:`1`
              (bind (_state_3 _optionindex_3) (`self.AddDialogue` "Volunteer" "Yeah she's a real class act that one and her kid isn’t any better. She spent pretty much all day yesterday treating the volunteers like they were her personal servants and the kid was treating the entire space like he owned it. We got a bunch of complaints about his behavior but his mom seemed more interested in telling off all the cosplayers instead of handling her kid. If they keep it up today I’ll make sure to remove them from the space myself." (`|MakeArray` "Sorry. Yesterday must have been brutal" :!type "Text")))
              (switch `/Game/Blueprint/Enum_DiaState` _state_3
                (:`NewEnumerator0`
                  (switch `int` _optionindex_3
                    (:`0`
                      (`self.CloseConversation`))))))
            (:`2`
              (bind (_state_4 _optionindex_4) (`self.AddDialogue` "Volunteer" "You and me both! I fully expected them to close down but the coordinators said something about being in too deep and not being able to afford mass refunds from patrons and vendors so here we are. Weird being this close to where a body was just a few hours ago." (`|MakeArray` "Your telling me. Hopefully we can put this case to rest and get home fast." :!type "Text")))
              (switch `/Game/Blueprint/Enum_DiaState` _state_4
                (:`NewEnumerator0`
                  (switch `int` _optionindex_4
                    (:`0`
                      (`self.CloseConversation`))))))
            (:`3`
              (bind (_state_5 _optionindex_5) (`self.AddDialogue` "Volunteer" "How can i help" (`|MakeArray` "Just passing thru" :!type "Text")))
              (switch `/Game/Blueprint/Enum_DiaState` _state_5
                (:`NewEnumerator0`
                  (switch `int` _optionindex_5
                    (:`0`
                      (goto _label))))))))))))