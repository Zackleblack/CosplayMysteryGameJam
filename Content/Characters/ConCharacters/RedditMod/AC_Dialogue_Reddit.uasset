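; Dialogue component for Redee, a convention-going figure collector the player questions about Yo-Yo's death.
; DialogueTreeIndex selects the first afternoon, first evening or second afternoon conversation, each built from nested AddDialogue calls branching on the chosen option; index 2 has no branch.
; Updated states on key replies set RedditToVendor and RedditToSecond on the first-person character.
; The last conversation reveals a discarded phone, then closes and shows the W_Movie widget.
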(fn `Dialogue`
  (`parent.Dialogue`)
  (set `self.DialogueIndex` -1)
  (switch `int` (`self.DialogueTreeIndex`)
    (:`0`
      ; 1Afternoon
      (bind (_state _optionindex) (`self.AddDialogue` "Redee" "Ahh, I see I've been approached by an officer of the courts. How may I be of assistance?" (`|MakeArray` "Where were you last night?" :!type "Text")))
      (switch `/Game/Blueprint/Enum_DiaState` _state
        (:`NewEnumerator0`
          (switch `int` _optionindex
            (:`0`
              (bind (_state_2 _optionindex_2) (`self.AddDialogue` "Redee" "Erm, last night I was waiting in line at Vincents to pick up the new Miku Figure. They released versions specifically for this convention and I had to have them to join my sealed collection." (`|MakeArray` "Was anybody there to witness that?" "That must have cost a fortune!" :!type "Text")))
              (switch `/Game/Blueprint/Enum_DiaState` _state_2
                (:`NewEnumerator0`
                  (switch `int` _optionindex_2
                    (:`0`
                      (bind (_state_3 _optionindex_3) (`self.AddDialogue` "Redee" "If you must know, Vincent sold me the figure so he would know I was there. So you can go talk to him if you absolutely must." (`|MakeArray` "I'll do that" :!type "Text")))
                      (switch `/Game/Blueprint/Enum_DiaState` _state_3
                        (:`NewEnumerator0`
                          (switch `int` _optionindex_3
                            (:`0`
                              (`self.CloseConversation` :!label _label))))
                        (:`NewEnumerator1`
                          (bind _asbp_first_person_character (cast `/Game/FirstPerson/Blueprints/BP_FirstPersonCharacter` (`GameplayStatics.GetPlayerPawn` 0)))
                          (set `/Game/FirstPerson/Blueprints/BP_FirstPersonCharacter.RedditToVendor` true _asbp_first_person_character))))
                    (:`1`
                      (bind (_state_4 _optionindex_4) (`self.AddDialogue` "Redee" "Heh, unlike some amature collectors here I have saved up for this con for months so I could spare no expense when it comes to acquiring these lovely ladies for my collection!" (`|MakeArray` "…alright then." :!type "Text")))
                      (switch `/Game/Blueprint/Enum_DiaState` _state_4
                        (:`NewEnumerator0`
                          (switch `int` _optionindex_4
                            (:`0`
                              (goto _label))))))))))))))
    (:`1`
      ; 1Evening
      (bind (_state_5 _optionindex_5) (`self.AddDialogue` "Redee" "*tips fedora* I take it you have some news from the front" (`|MakeArray` "I spoke with the vendor and he remembers you asking about a sold out figure that Yo-Yo Mon got the last one of before you ran over to where she was." "After purchasing the figure yesterday what did you do afterwards?" :!type "Text")))
      (switch `/Game/Blueprint/Enum_DiaState` _state_5
        (:`NewEnumerator0`
          (switch `int` _optionindex_5
            (:`0`
              (bind (_state_6 _optionindex_6) (`self.AddDialogue` "Redee" "You think I would sully my hands over an incomplete collection? I am a passionate lover of the arts and would never bring harm to any of its muses. I got out of there quickly because I had other obligations to attend to. I wanted to try and get in line quickly for Yo-yo's meet and greet but the line was too long so I went over to Sparkle's booth since her line was much shorter" (`|MakeArray` "I'll talk with Sparkles" :!type "Text")))
              (switch `/Game/Blueprint/Enum_DiaState` _state_6
                (:`NewEnumerator0`
                  (switch `int` _optionindex_6
                    (:`0`
                      (`self.CloseConversation` :!label _label_2))))
                (:`NewEnumerator1`
                  (bind _asbp_first_person_character_2 (cast `/Game/FirstPerson/Blueprints/BP_FirstPersonCharacter` (`GameplayStatics.GetPlayerPawn` 0)))
                  (set `/Game/FirstPerson/Blueprints/BP_FirstPersonCharacter.RedditToSecond` true _asbp_first_person_character_2))))
            (:`1`
              (bind (_state_7 _optionindex_7) (`self.AddDialogue` "Redee" "I had a meet and greet session with Yo-yo but I never got the chance. The line was too long and they started closing the hall before I got to the front. " (`|MakeArray` "I'm sorry to hear that" :!type "Text")))
              (switch `/Game/Blueprint/Enum_DiaState` _state_7
                (:`NewEnumerator0`
                  (switch `int` _optionindex_7
                    (:`0`
                      (goto _label_2))))))))))
    (:`3`
      ; 2Afternoon
      (bind (_state_8 _optionindex_8) (`self.AddDialogue` "Redee" "*you notice his pheromones are maxed*" (`|MakeArray` "Where were you? We didn’t see you around this morning and you look...uh...dirty" :!type "Text")))
      (switch `/Game/Blueprint/Enum_DiaState` _state_8
        (:`NewEnumerator0`
          (switch `int` _optionindex_8
            (:`0`
              (bind (_state_9 _optionindex_9) (`self.AddDialogue` "Redee" "Many apologies, I went looking through the dumpster with the hopes of retrieving the late Yo-yo’s exclusive Miku figure. I understand it was in poor taste to do so but the idea of her sitting in a trash pile bothered me. I did find something useful though. Someone tossed out a phone. Seems rather fortuitous that a gentlesir such as myself stumbled upon such an ideal piece of evidence" (`|MakeArray` "That's great. This could be helpful in figuring out what happened!" :!type "Text")))
              (switch `/Game/Blueprint/Enum_DiaState` _state_9
                (:`NewEnumerator0`
                  (switch `int` _optionindex_9
                    (:`0`
                      (`self.CloseConversation`)
                      (bind _returnvalue (`|CreateWidget` "/Game/Widgets/W_Movie.W_Movie_C"))
                      (`UserWidget.AddToViewport` _returnvalue 0))))))))))))