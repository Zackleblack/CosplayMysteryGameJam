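; BP_Redditmod is an interactable NPC character that holds a Reddit-themed dialogue conversation with the first-person player.
; On interact, it copies the player's dialogue tree index into its own Reddit dialogue component and opens the conversation.
; Every tick it hides its plane when the player's index equals two, otherwise shows it.
; A name label, set at construction, appears only while the character is interactable.
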(event `self.ReceiveTick`
  (params (DeltaSeconds :type "Float (single-precision)"))
  (bind _asbp_first_person_character (cast `/Game/FirstPerson/Blueprints/BP_FirstPersonCharacter` (`GameplayStatics.GetPlayerPawn` 0)))
  (if (== (`/Game/Blueprint/AC_Dialogue_Base.DialogueTreeIndex` (`/Game/FirstPerson/Blueprints/BP_FirstPersonCharacter.AC_Dialogue_Base` _asbp_first_person_character)) 2)
    (`SceneComponent.SetVisibility` (`self.Plane`) false false)
    (else
      (`SceneComponent.SetVisibility` (`self.Plane`) true false))))

(event `/Game/Blueprint/BPI_Interact.SetInteractableState`
  (params (bCanShowInteract :type Boolean))
  (if bCanShowInteract
    (`SceneComponent.SetVisibility` (`self.Txt Ch Name`) true false)
    (else
      (`SceneComponent.SetVisibility` (`self.Txt Ch Name`) false false))))

(event `/Game/Blueprint/BPI_Interact.Interact`
  (params (Instigator :type "Actor Object Reference"))
  (bind _output_get (set `self.Intergator` Instigator))
  (bind _asbp_first_person_character (cast `/Game/FirstPerson/Blueprints/BP_FirstPersonCharacter` _output_get))
  (set `/Game/Blueprint/AC_Dialogue_Base.DialogueTreeIndex` (`/Game/Blueprint/AC_Dialogue_Base.DialogueTreeIndex` (`/Game/FirstPerson/Blueprints/BP_FirstPersonCharacter.AC_Dialogue_Base` _asbp_first_person_character)) (`self.AC_Dialogue_Reddit`))
  (`/Game/Blueprint/AC_Dialogue_Base.OpenConversation` (`self.AC_Dialogue_Reddit`)))

(fn `UserConstructionScript`
  (`TextRenderComponent.K2_SetText` (`self.Txt Ch Name`) (`self.CharacterName`)))