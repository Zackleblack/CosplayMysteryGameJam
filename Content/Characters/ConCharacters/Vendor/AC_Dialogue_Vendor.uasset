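; Dialogue component for the convention Vendor NPC, who gives witness testimony in a murder investigation.
; Its Dialogue function overrides the parent and builds a branching tree from chained AddDialogue calls, switching on the returned state and chosen option index.
; The player character's RedditToVendor flag unlocks the questioning options, including leads on a suspicious figure buyer.
; Each completed branch ends by closing the conversation.
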(fn `Dialogue`
  (`parent.Dialogue`)
  (set `self.DialogueIndex` -1)
  (switch `int` (`self.DialogueTreeIndex`)
    (:`0`
      (cast `/Game/FirstPerson/Blueprints/BP_FirstPersonCharacter` (`GameplayStatics.GetPlayerPawn` 0))
      (bind _asbp_first_person_character (cast `/Game/FirstPerson/Blueprints/BP_FirstPersonCharacter` (`GameplayStatics.GetPlayerPawn` 0)))
      (bind (_state _optionindex) (`self.AddDialogue` "Vendor" "See anything you like?" (select `bool` (`/Game/FirstPerson/Blueprints/BP_FirstPersonCharacter.RedditToVendor` _asbp_first_person_character) :`false` (`|MakeArray` "Just looking thanks!" :!type "Text") :`true` (`|MakeArray` "Just looking thanks!" "Were you here after hours at all?" "Did you see anything that looked out of place?" "Do you remember selling a figure to this guy last night? *Produces picture*" :!type "Text"))))
      (switch `/Game/Blueprint/Enum_DiaState` _state
        (:`NewEnumerator0`
          (switch `int` _optionindex
            (:`0`
              (`self.CloseConversation` :!label _label))
            (:`1`
              (bind (_state_2 _optionindex_2) (`self.AddDialogue` "Vendor" "None of us vendors were here. We left right around closing as we had a dinner reservation downtown for the staff." (`|MakeArray` "Continue" :!type "Text")))
              (switch `/Game/Blueprint/Enum_DiaState` _state_2
                (:`NewEnumerator0`
                  (switch `int` _optionindex_2
                    (:`0`
                      (goto _label))))))
            (:`2`
              (bind (_state_3 _optionindex_3) (`self.AddDialogue` "Vendor" "There was one thing, though it was more annoying than suspicious. There was some kid with a selfie stick running around loudly filming stuff. I don’t see him around, though I can't say I’m upset about that. It's sad that it took a murder to get some peace and quiet though." (`|MakeArray` "Continue" :!type "Text")))
              (switch `/Game/Blueprint/Enum_DiaState` _state_3
                (:`NewEnumerator0`
                  (switch `int` _optionindex_3
                    (:`0`
                      (`self.CloseConversation`))))))
            (:`3`
              (bind (_state_4 _optionindex_4) (`self.AddDialogue` "Vendor" "Yea he was a strange character. I could barely get through a conversation with him because he was either ogling the cosplayers or arguing with other patrons in line. Almost had to ask him to leave but he eventually reached the front of the line, asked a few questions, made his purchase, and then took off in a hurry." (`|MakeArray` "Where did he run off to?" "What questions did he ask?" :!type "Text")))
              (switch `/Game/Blueprint/Enum_DiaState` _state_4
                (:`NewEnumerator0`
                  (switch `int` _optionindex_4
                    (:`0`
                      (bind (_state_5 _optionindex_5) (`self.AddDialogue` "Vendor" "I don't know for sure since I had to move on to helping the next customer, but it was in the direction of the cosplayers tables." (`|MakeArray` "I'll look into it." "" :!type "Text")))
                      (switch `/Game/Blueprint/Enum_DiaState` _state_5
                        (:`NewEnumerator0`
                          (switch `int` _optionindex_5
                            (:`0`
                              _)))))
                    (:`1`
                      (bind (_state_6 _optionindex_6) (`self.AddDialogue` "Vendor" "He asked about a limited edition figure. We got two different ones for this convention that are exclusive. We had already sold the last one for one of them a few hours ago to Yo-Yo Mon. Poor girl, I doubt she even got to take the figure out of the box" (`|MakeArray` "I'll look into it." "" :!type "Text")))
                      (switch `/Game/Blueprint/Enum_DiaState` _state_6
                        (:`NewEnumerator0`
                          (switch `int` _optionindex_6
                            (:`0`
                              _))))))
                  (`self.CloseConversation`))))))))))