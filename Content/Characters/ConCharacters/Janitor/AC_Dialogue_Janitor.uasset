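; Dialogue component for the Janitor character, holding his conversations in a murder investigation around a convention cosplay contestant, Second Place.
; Overrides Dialogue, resets DialogueIndex, then switches on DialogueTreeIndex to pick a conversation: initial questioning, idle greeting, follow-up confrontation, or evidence-found resolution.
; Each tree nests AddDialogue calls that branch on the chosen option and end in CloseConversation.
; In the confrontation, one of two replies draws out his confession.
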(fn `Dialogue`
  (`parent.Dialogue`)
  (set `self.DialogueIndex` -1)
  (switch `int` (`self.DialogueTreeIndex`)
    (:`0`
      (bind (_state _optionindex) (`self.AddDialogue` "Janitor" "Can I help you?" (`|MakeArray` "Did you happen to see anybody suspicious back here after hours?" :!type "Text")))
      (switch `/Game/Blueprint/Enum_DiaState` _state
        (:`NewEnumerator0`
          (switch `int` _optionindex
            (:`0`
              (bind (_state_2 _optionindex_2) (`self.AddDialogue` "Janitor" "No, the only people back here were myself and some of the other cleaning staff" (`|MakeArray` "Did you clean back here?" :!type "Text")))
              (switch `/Game/Blueprint/Enum_DiaState` _state_2
                (:`NewEnumerator0`
                  (switch `int` _optionindex_2
                    (:`0`
                      (bind (_state_3 _optionindex_3) (`self.AddDialogue` "Janitor" "No, I haven’t touched anything back here. I was actually just now coming back here to do some morning cleaning but it looks like someone beat me to it. Not that I’m complaining, it means one less thing for me to do at the end of the day." (`|MakeArray` "Thank you, sorry for bothering you." :!type "Text")))
                      (switch `/Game/Blueprint/Enum_DiaState` _state_3
                        (:`NewEnumerator0`
                          (switch `int` _optionindex_3
                            (:`0`
                              (`self.CloseConversation`))))))))))))))
    (:`1`
      (bind (_state_4 _optionindex_4) (`self.AddDialogue` "Janitor" "Can I help you?" (`|MakeArray` "Just passing thru" :!type "Text")))
      (switch `/Game/Blueprint/Enum_DiaState` _state_4
        (:`NewEnumerator0`
          (switch `int` _optionindex_4
            (:`0`
              (`self.CloseConversation`))))))
    (:`2`
      (bind (_state_5 _optionindex_5) (`self.AddDialogue` "Janitor" "Can I help you?" (`|MakeArray` "I’d like to ask you some more questions in regards to the night of the incident, specifically to whether the room was cleaned or not" :!type "Text")))
      (switch `/Game/Blueprint/Enum_DiaState` _state_5
        (:`NewEnumerator0`
          (switch `int` _optionindex_5
            (:`0`
              (bind (_state_6 _optionindex_6) (`self.AddDialogue` "Janitor" "Look I already told you, I wasn’t here. I didn’t clean the night of the murder. Instead of hounding me about it if you really want to help go question Second Place. She was the one in here last." (`|MakeArray` "I did, she insists that she was in here fixing her cosplay yet the proof that she did so was thrown out. It wouldn’t make sense for her to have thrown away her only solid alibi." " I did, she seems to think that you're lying and I believe her. I think you know more than you're telling us. If you don’t speak up now an innocent person could go to jail. " :!type "Text")))
              (switch `/Game/Blueprint/Enum_DiaState` _state_6
                (:`NewEnumerator0`
                  (switch `int` _optionindex_6
                    (:`0`
                      (bind (_state_7 _optionindex_7) (`self.AddDialogue` "Janitor" "Well even if she didn’t do it that doesn’t mean I was in here to do it either. I don't know what to tell you, now leave me alone." (`|MakeArray` "Continue" :!type "Text")))
                      (switch `/Game/Blueprint/Enum_DiaState` _state_7
                        (:`NewEnumerator0`
                          (switch `int` _optionindex_7
                            (:`0`
                              (`self.CloseConversation`))))))
                    (:`1`
                      (bind (_state_8 _optionindex_8) (`self.AddDialogue` "Janitor" "Ok ok, look I was in here and I cleaned up alright. I'm on parole and I really don’t want to be tied up in all this mess. Trash hasn’t run yet so I’ll go looking for the item in the dumpster but in return you need to leave my name out of this. Meet me back here this afternoon and I’ll let you know what I find" (`|MakeArray` "Continue" :!type "Text")))
                      (switch `/Game/Blueprint/Enum_DiaState` _state_8
                        (:`NewEnumerator0`
                          (switch `int` _optionindex_8
                            (:`0`
                              (`self.CloseConversation`))))))))))))))
    (:`3`
      (bind (_state_9 _optionindex_9) (`self.AddDialogue` "Janitor" "I was able to find Second Place’s cosplay piece in the dumpster. I was thinking about what you said and I can’t in good conscience let an innocent person take the fall so I tipped off the police and am willing to testify in her defense. I just hope my parole officer doesn’t get too spooked that I’m this close to a crime scene and trusts that I had nothing to do with it." (`|MakeArray` "Thank you. She will appreciate this greatly" :!type "Text")))
      (switch `/Game/Blueprint/Enum_DiaState` _state_9
        (:`NewEnumerator0`
          (switch `int` _optionindex_9
            (:`0`
              (`self.CloseConversation`))))))))