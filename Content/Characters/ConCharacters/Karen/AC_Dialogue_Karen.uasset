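; Dialogue component for Karen, a convention-goer in a murder mystery, also voicing her son Chad under her speaker name.
; The Dialogue override calls the parent, resets DialogueIndex, then picks one of four day and time conversations by DialogueTreeIndex.
; Nested AddDialogue calls branch on the chosen option and end in CloseConversation.
; The player character's SpokeFan flag unlocks an extra question on the first afternoon.
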(fn `Dialogue`
  (`parent.Dialogue`)
  (set `self.DialogueIndex` -1)
  (switch `int` (`self.DialogueTreeIndex`)
    (:`0`
      ; 1Afternoon
      (bind (_state _optionindex) (`self.AddDialogue` "Karen" "Be a dear and fetch us some waters please. Sparkling preferred" (`|MakeArray` "Where were you last night?" :!type "Text")))
      (switch `/Game/Blueprint/Enum_DiaState` _state
        (:`NewEnumerator0`
          (switch `int` _optionindex
            (:`0`
              (bind _asbp_first_person_character (cast `/Game/FirstPerson/Blueprints/BP_FirstPersonCharacter` (`GameplayStatics.GetPlayerPawn` 0)))
              (bind (_state_2 _optionindex_2) (`self.AddDialogue` "Karen" "Back in our hotel room with my son obviously. There are too many scantily clad harlots walking around here at night and I'm not about to expose him to such low life filth at his impressionable age." (select `bool` (`/Game/FirstPerson/Blueprints/BP_FirstPersonCharacter.SpokeFan` _asbp_first_person_character) :`false` (`|MakeArray` "If you have such an issue with cosplayers what brings you out to Con Spiracy?" "Those “harlots” are people too, and one of them was just killed!" :!type "Text") :`true` (`|MakeArray` "If you have such an issue with cosplayers what brings you out to Con Spiracy?" "Those “harlots” are people too, and one of them was just killed!" "Someone saw you arguing with the volunteers earlier. What was that about?" :!type "Text"))))
              (switch `/Game/Blueprint/Enum_DiaState` _state_2
                (:`NewEnumerator0`
                  (switch `int` _optionindex_2
                    (:`0`
                      (bind (_state_3 _optionindex_3) (`self.AddDialogue` "Karen" "*sigh*, My son loves this stuff and as much as I hate it. Besides, I read in a recent issue of Fair Parent Magazine he should be free to explore his interests. I just hope he comes to his senses soon and moves past this phase. Though with how much he's on his phone and filming everything I doubt that will happen." (`|MakeArray` "Where is your son? I don't see him here with you." "Good on you! You seem like a good parent for that." :!type "Text")))
                      (switch `/Game/Blueprint/Enum_DiaState` _state_3
                        (:`NewEnumerator0`
                          (switch `int` _optionindex_3
                            (:`0`
                              (bind (_state_4 _optionindex_4) (`self.AddDialogue` "Karen" "I sent him back up to our room while this is all going on. If I don't want him around *those* people I absolutely don't want to tarnish his innocent mind by having him here at a crime scene." (`|MakeArray` "That makes sense really." :!type "Text")))
                              (switch `/Game/Blueprint/Enum_DiaState` _state_4
                                (:`NewEnumerator0`
                                  (switch `int` _optionindex_4
                                    (:`0`
                                      _)))))
                            (:`1`
                              (bind (_state_5 _optionindex_5) (`self.AddDialogue` "Karen" "Thank you, finally another reasonable person here. Just between you and me, there seemed to be some kind of tension between those two in the cosplay contest before one of them got killed. That lizard costume is just too creepy to not be suspicious." (`|MakeArray` "I'll look into that. Thanks!" :!type "Text")))
                              (switch `/Game/Blueprint/Enum_DiaState` _state_5
                                (:`NewEnumerator0`
                                  (switch `int` _optionindex_5
                                    (:`0`
                                      _)))))))))
                    (:`1`
                      (bind (_state_6 _optionindex_6) (`self.AddDialogue` "Karen" "Well, excuse me for having my opinion on the matter and protecting my son. If someone as rude as you is defending them, maybe that death was justified! Hmph! \n" (`|MakeArray` "HMPH!!" :!type "Text")))
                      (switch `/Game/Blueprint/Enum_DiaState` _state_6
                        (:`NewEnumerator0`
                          (switch `int` _optionindex_6
                            (:`0`
                              _)))))
                    (:`2`
                      (bind (_state_7 _optionindex_7) (`self.AddDialogue` "Karen" "Well if you must know, the people here are awful and cant do basic things I ask for right. Chad wanted his backup selfie stick, I told them to get that from our room and they refused to!!! Something about “we don't know what room” and “we cant enter guests spaces” and “We are volunteers, not staff”. All that sounds like  excuses to be lazy to me." (`|MakeArray` "How charming..." :!type "Text")))
                      (switch `/Game/Blueprint/Enum_DiaState` _state_7
                        (:`NewEnumerator0`
                          (switch `int` _optionindex_7
                            (:`0`
                              _))))))
                  (`self.CloseConversation`))))))))
    (:`1`
      ; 1Evening
      (bind (_state_8 _optionindex_8) (`self.AddDialogue` "Karen" "Chad! Say hi to the nice fake investigator!" (`|MakeArray` "What have you been up to?" "Why were you not here earlier?" "What is that you're holding?" :!type "Text")))
      (switch `/Game/Blueprint/Enum_DiaState` _state_8
        (:`NewEnumerator0`
          (switch `int` _optionindex_8
            (:`0`
              (bind (_state_9 _optionindex_9) (`self.AddDialogue` "Karen" "Obviously recording all of this for my fans online! There isn't a moment or angle of this I want to miss so I've been running around filming it all. They eat this anime stuff up." (`|MakeArray` "Do you have any of the footage I can look at?" "Did you see anyone weird while running around?" :!type "Text")))
              (switch `/Game/Blueprint/Enum_DiaState` _state_9
                (:`NewEnumerator0`
                  (switch `int` _optionindex_9
                    (:`0`
                      (bind (_state_10 _optionindex_10) (`self.AddDialogue` "Karen" "The vid isn't done, so obviously no. Plus my phone is missing so even if I did want to, I can't. But you can follow me on Punch and MeToob to see it once it's done" (`|MakeArray` "I see. Well if you find it, it could be important!" :!type "Text")))
                      (switch `/Game/Blueprint/Enum_DiaState` _state_10
                        (:`NewEnumerator0`
                          (switch `int` _optionindex_10
                            (:`0`
                              _)))))
                    (:`1`
                      (bind (_state_11 _optionindex_11) (`self.AddDialogue` "Karen" "Yeah bro, that janitor dude was looking around a bunch after leaving the backstage area and left quickly. Low key may be a lead you can follow… or a follow up story I can film!" (`|MakeArray` "I'll keep you and your followers posted" :!type "Text")))
                      (switch `/Game/Blueprint/Enum_DiaState` _state_11
                        (:`NewEnumerator0`
                          (switch `int` _optionindex_11
                            (:`0`
                              _)))))))))
            (:`1`
              (bind (_state_12 _optionindex_12) (`self.AddDialogue` "Karen" "If you want to be mad at someone blame my LAME mom. She didn't want me to be “surrounded by a murder and poor Influences” as if that wouldn’t have been the most RAD twist for my vlog. Plus it's not like I haven't seen this stuff in videogames before." (`|MakeArray` "Im sure she was just worried for your safetly" :!type "Text")))
              (switch `/Game/Blueprint/Enum_DiaState` _state_12
                (:`NewEnumerator0`
                  (switch `int` _optionindex_12
                    (:`0`
                      _)))))
            (:`2`
              (bind (_state_13 _optionindex_13) (`self.AddDialogue` "Karen" "It’s the X-2 triple fold titanium stainless steel premium vlogging and selfie stick. Not that I’m using it for much right now since I’m not supposed to be filming this. At least I can do tricks with it and pretend it's a sword or something!" (`|MakeArray` "Well be careful swinging that around. You could seriously hurt someone!" :!type "Text")))
              (switch `/Game/Blueprint/Enum_DiaState` _state_13
                (:`NewEnumerator0`
                  (switch `int` _optionindex_13
                    (:`0`
                      _))))))
          (`self.CloseConversation`))))
    (:`2`
      ; 2Morning
      (bind (_state_14 _optionindex_14) (`self.AddDialogue` "Karen" "Chad! Say hi to the nice fake investigator!" (`|MakeArray` "(to kid) where is your phone?" "(to parent) Have you seen anything unusual this morning?" :!type "Text")))
      (switch `/Game/Blueprint/Enum_DiaState` _state_14
        (:`NewEnumerator0`
          (switch `int` _optionindex_14
            (:`0`
              (bind _state_15 (`self.AddDialogue` "Karen" "So, you won't believe this, the craziest thing happened the other day and I lost it. Sucks right?! Kinda didn't want to bring it up till now because the one thing worse than losing that sick footage is getting grounded." (`|MakeArray` "Continue" :!type "Text")))
              (switch `/Game/Blueprint/Enum_DiaState` _state_15
                (:`NewEnumerator0`
                  (switch `int` 0
                    (:`0`
                      (bind _state_16 (`self.AddDialogue` "Karen" "(Mom) Which you most definitely are as soon as we get home! First these anime womens and now this. Since you're already searching around, if you come across the phone will you let us know?" (`|MakeArray` "Yes Ma'am" :!type "Text")))
                      (switch `/Game/Blueprint/Enum_DiaState` _state_16
                        (:`NewEnumerator0`
                          (switch `int` 0
                            (:`0`
                              _)))))))))
            (:`1`
              (bind _state_17 (`self.AddDialogue` "Karen" "Well, that excitable girl seems a little too excitable today. Don't get me wrong I am not too upset at this whole ordeal besides it being an inconvenience to my schedule. But even I wouldn't be as excited as she is." (`|MakeArray` "I'll see whats got her so giddy" :!type "Text")))
              (switch `/Game/Blueprint/Enum_DiaState` _state_17
                (:`NewEnumerator0`
                  (switch `int` 0
                    (:`0`
                      _))))))
          (`self.CloseConversation`))))
    (:`3`
      ; 2Afternoon
      (bind (_state_18 _optionindex_15) (`self.AddDialogue` "Karen" "Chad! Say hi to the nice fake investigator!" (`|MakeArray` "Cherryl, always a “pleasure” to see you" "Greetings your highness *bows*" :!type "Text")))
      (switch `/Game/Blueprint/Enum_DiaState` _state_18
        (:`NewEnumerator0`
          (switch `int` _optionindex_15
            (:`0`
              _)
            (:`1`
              _))
          (bind (_state_19 _optionindex_16) (`self.AddDialogue` "Karen" "I'm sorry to interrupt what I'm sure was a well rehearsed quip but I'm in the middle of trying to track down my son's phone. While we do have extra’s to spare it gets tiring having to replace them so frequently and none of these attendants seem keen on helping procure it." (`|MakeArray` "Why isn’t your son helping track it down? It was his after all." :!type "Text")))
          (switch `/Game/Blueprint/Enum_DiaState` _state_19
            (:`NewEnumerator0`
              (switch `int` _optionindex_16
                (:`0`
                  (bind (_state_20 _optionindex_17) (`self.AddDialogue` "Karen" "He seems rather content with it not being found at all. He seems to think that every time he loses or breaks something it can just be instantly replaced." (`|MakeArray` "Can't imagine where he would have picked that up from" :!type "Text")))
                  (switch `/Game/Blueprint/Enum_DiaState` _state_20
                    (:`NewEnumerator0`
                      (switch `int` _optionindex_17
                        (:`0`
                          (`self.CloseConversation`))))))))))))))