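; Dialogue component for Sparkles, a cosplayer and rival of the murder victim, whom the player questions as a suspect.
; Its Dialogue override picks a branching conversation by DialogueTreeIndex, covering afternoon and evening of day one, then morning and evening of day two.
; First-person character flags alter options, and choices set SecondShutDown, which replaces all later talk with a rebuff, or JanitorConvince.
; The node setting FindtheEye is unconnected, so it never runs.
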(fn `Dialogue`
  (`parent.Dialogue`)
  (set `self.DialogueIndex` -1)
  (bind _asbp_first_person_character (cast `/Game/FirstPerson/Blueprints/BP_FirstPersonCharacter` (`GameplayStatics.GetPlayerPawn` 0)))
  (if (`/Game/FirstPerson/Blueprints/BP_FirstPersonCharacter.SecondShutDown` _asbp_first_person_character)
    (bind (_state _optionindex) (`self.AddDialogue` "Sparkles" "Get away from me!!" (`|MakeArray` "Continue" :!type "Text")))
    (switch `/Game/Blueprint/Enum_DiaState` _state
      (:`NewEnumerator0`
        (switch `int` _optionindex
          (:`0`
            (`self.CloseConversation`)))))
    (else
      (switch `int` (`self.DialogueTreeIndex`)
        (:`0`
          ; 1Afternoon
          (bind (_state_2 _optionindex_2) (`self.AddDialogue` "Sparkles" "Its so sad to think that shes gone...." (`|MakeArray` "Where were you last night?" "How did you know the victim?" :!type "Text")))
          (switch `/Game/Blueprint/Enum_DiaState` _state_2
            (:`NewEnumerator0`
              (switch `int` _optionindex_2
                (:`0`
                  (bind (_state_3 _optionindex_3) (`self.AddDialogue` "Sparkles" "I was in the dressing room fixing my cosplay. Of course it had to break minutes before the contest just like last time." (`|MakeArray` "Was anybody there to witness that?" "Oh no! What broke?" :!type "Text")))
                  (switch `/Game/Blueprint/Enum_DiaState` _state_3
                    (:`NewEnumerator0`
                      (switch `int` _optionindex_3
                        (:`0`
                          (bind (_state_4 _optionindex_4) (`self.AddDialogue` "Sparkles" "Not at the time no. I wasn’t exactly looking for witnesses at that moment, and everyone else was already on stage showing off their costumes." (`|MakeArray` "That does make things difficult" :!type "Text")))
                          (switch `/Game/Blueprint/Enum_DiaState` _state_4
                            (:`NewEnumerator0`
                              (switch `int` _optionindex_4
                                (:`0`
                                  (`self.CloseConversation`))))))
                        (:`1`
                          (bind (_state_5 _optionindex_5) (`self.AddDialogue` "Sparkles" "The pupil of my eye broke off. I had to take a marker and draw a temporary one on real quick. The old felt piece might still be in the dressing room" (`|MakeArray` "I'll go take a look!" :!type "Text")))
                          (switch `/Game/Blueprint/Enum_DiaState` _state_5
                            (:`NewEnumerator0`
                              (switch `int` _optionindex_5
                                (:`0`
                                  (`self.CloseConversation`))))
                            (:`NewEnumerator1`
                              (bind _asbp_first_person_character_2 (cast `/Game/FirstPerson/Blueprints/BP_FirstPersonCharacter` (`GameplayStatics.GetPlayerPawn` 0))))))))))
                (:`1`
                  (bind (_state_6 _optionindex_6) (`self.AddDialogue` "Sparkles" "We’ve collabed a few times on different projects. We didn’t always see eye to eye on everything but we were amicable even if just for business sake." (`|MakeArray` "What did you two argue about?" "What kind of projects?" :!type "Text")))
                  (switch `/Game/Blueprint/Enum_DiaState` _state_6
                    (:`NewEnumerator0`
                      (switch `int` _optionindex_6
                        (:`0`
                          (bind (_state_7 _optionindex_7) (`self.AddDialogue` "Sparkles" "Only a few things I guess. Who to cosplay, what collaborations to do, what materials to use, stitching techniques, where we should compete…That list sounds a lot longer now that I am saying it out loud." (`|MakeArray` "Im sure you  guys cared about each other very much." :!type "Text")))
                          (switch `/Game/Blueprint/Enum_DiaState` _state_7
                            (:`NewEnumerator0`
                              (switch `int` _optionindex_7
                                (:`0`
                                  _)))))
                        (:`1`
                          (bind (_state_8 _optionindex_8) (`self.AddDialogue` "Sparkles" "Nothing too special, mainly a few ships and duos. Speaking of which, that girl Phann seemed really obsessed with asking about a cosplay we used to do together. It's not much, but maybe you should talk to her to learn more about Yo-Yo Mon" (`|MakeArray` "I'll do that, thanks." :!type "Text")))
                          (switch `/Game/Blueprint/Enum_DiaState` _state_8
                            (:`NewEnumerator0`
                              (switch `int` _optionindex_8
                                (:`0`
                                  _))))))
                      (`self.CloseConversation`))))))))
        (:`1`
          ; 1Evening
          (bind (_state_9 _optionindex_9) (`self.AddDialogue` "Sparkles" "Any luck?" (`|MakeArray` "I looked around the dressing room and couldn't find anything back there, and the  janitor insisted that they hadn’t done any cleaning in the room yet." "The room was cleaned before we could get back there to check it. Do you have anything else we could use to clear your name?" :!type "Text")))
          (switch `/Game/Blueprint/Enum_DiaState` _state_9
            (:`NewEnumerator0`
              (switch `int` _optionindex_9
                (:`0`
                  (bind (_state_10 _optionindex_10) (`self.AddDialogue` "Sparkles" "Are you insinuating that I'm lying? You seriously believe some janitor nobody over me when you're clearly the problem and didn't search hard enough. You got some nerve walking around her in your low budget cosplay accusing me of something so disgusting." (`|MakeArray` "OBJECTION!!" :!type "Text")))
                  (switch `/Game/Blueprint/Enum_DiaState` _state_10
                    (:`NewEnumerator0`
                      (switch `int` _optionindex_10
                        (:`0`
                          _)))))
                (:`1`
                  (bind (_state_11 _optionindex_11) (`self.AddDialogue` "Sparkles" "Not really. I wasn’t trying to prepare an alibi because I didn’t think one would be needed. I really didn't have a reason to get rid of her. Sure we were rivals but I always viewed it as a healthy, friendly rivalry. We lifted each other up and kept pushing each other forward. She was as much a friend as she was a rival. " (`|MakeArray` "Can you think of someone who would do this?" "Did you see anyone else enter backstage between you and the janitor?" :!type "Text")))
                  (switch `/Game/Blueprint/Enum_DiaState` _state_11
                    (:`NewEnumerator0`
                      (switch `int` _optionindex_11
                        (:`0`
                          (bind (_state_12 _optionindex_12) (`self.AddDialogue` "Sparkles" "That mom with the kid seems a bit off to me. I’m glad the kid is here now incase he knows something, but the way the mom keeps looking at me gives me bad vibes." (`|MakeArray` "I guess I'll go chat them up" :!type "Text")))
                          (switch `/Game/Blueprint/Enum_DiaState` _state_12
                            (:`NewEnumerator0`
                              (switch `int` _optionindex_12
                                (:`0`
                                  _)))))
                        (:`1`
                          (bind (_state_13 _optionindex_13) (`self.AddDialogue` "Sparkles" "Nope, the only person to enter the room after me and before the  murder was the Janitor." (`|MakeArray` "I might have to pay him another visit" :!type "Text")))
                          (switch `/Game/Blueprint/Enum_DiaState` _state_13
                            (:`NewEnumerator0`
                              (switch `int` _optionindex_13
                                (:`0`
                                  _))))))))))
              (`self.CloseConversation`))))
        (:`2`
          (bind _asbp_first_person_character_3 (cast `/Game/FirstPerson/Blueprints/BP_FirstPersonCharacter` (`GameplayStatics.GetPlayerPawn` 0)))
          ; 2Morning
          (bind (_state_14 _optionindex_14) (`self.AddDialogue` "Sparkles" "I hope you have good news..." (select `bool` (`/Game/FirstPerson/Blueprints/BP_FirstPersonCharacter.RedditToSecond` _asbp_first_person_character_3) :`false` (`|MakeArray` "How are you holding up today?" :!type "Text") :`true` (`|MakeArray` "How are you holding up today?" "Reddit Mod said they spoke with you during your meet and greet. How was your interaction with him?" :!type "Text"))))
          (switch `/Game/Blueprint/Enum_DiaState` _state_14
            (:`NewEnumerator0`
              (switch `int` _optionindex_14
                (:`0`
                  (bind (_state_15 _optionindex_15) (`self.AddDialogue` "Sparkles" "In a word? Rough. I’ve been getting questioned by police all day and I told them the same thing I had told you. However, since the room was cleaned, and I wasn’t around anybody that late, I seem to have been placed as suspect number 1!" (`|MakeArray` "Well can you blame them? Given your last known location and relationship with them it does make sense." "For what it's worth I think you're innocent and I'm going to prove it!" :!type "Text")))
                  (switch `/Game/Blueprint/Enum_DiaState` _state_15
                    (:`NewEnumerator0`
                      (switch `int` _optionindex_15
                        (:`0`
                          (bind (_state_16 _optionindex_16) (`self.AddDialogue` "Sparkles" "Screw you! I don’t need this from you too! I know I didn’t do it and I don’t care what you or anybody else thinks!!" (`|MakeArray` "Continue" :!type "Text")))
                          (switch `/Game/Blueprint/Enum_DiaState` _state_16
                            (:`NewEnumerator0`
                              (switch `int` _optionindex_16
                                (:`0`
                                  (`self.CloseConversation` :!label _label))))
                            (:`NewEnumerator1`
                              (bind _asbp_first_person_character_4 (cast `/Game/FirstPerson/Blueprints/BP_FirstPersonCharacter` (`GameplayStatics.GetPlayerPawn` 0)))
                              (set `/Game/FirstPerson/Blueprints/BP_FirstPersonCharacter.SecondShutDown` true _asbp_first_person_character_4))))
                        (:`1`
                          (bind (_state_17 _optionindex_17) (`self.AddDialogue` "Sparkles" "Thank you so much. At least somebody is in my corner. Could you please question the janitorial staff again? I know you have already, but something just doesn't add up there for me. Surely somebody must know something!" (`|MakeArray` "Continue" :!type "Text")))
                          (switch `/Game/Blueprint/Enum_DiaState` _state_17
                            (:`NewEnumerator0`
                              (switch `int` _optionindex_17
                                (:`0`
                                  (goto _label))))
                            (:`NewEnumerator1`
                              (bind _asbp_first_person_character_5 (cast `/Game/FirstPerson/Blueprints/BP_FirstPersonCharacter` (`GameplayStatics.GetPlayerPawn` 0)))
                              (set `/Game/FirstPerson/Blueprints/BP_FirstPersonCharacter.JanitorConvince` true _asbp_first_person_character_5))))))))
                (:`1`
                  (bind (_state_18 _optionindex_18) (`self.AddDialogue` "Sparkles" "The guy with the body pillow? Yeah he was there. We talked a little and even took some photos together, nothing too out of the ordinary. Weirdly he did keep looking over at Yo-Yo Mon’s meet and greet while we talked. He didn't seem to be doing in a weird way though like I first thought. More like he was, sad Disappointed maybe?" (`|MakeArray` "Continue" :!type "Text")))
                  (switch `/Game/Blueprint/Enum_DiaState` _state_18
                    (:`NewEnumerator0`
                      (switch `int` _optionindex_18
                        (:`0`
                          (goto _label))))))))))
        (:`3`
          (bind _asbp_first_person_character_6 (cast `/Game/FirstPerson/Blueprints/BP_FirstPersonCharacter` (`GameplayStatics.GetPlayerPawn` 0)))
          ; 2Evening
          (bind (_state_19 _optionindex_19) (`self.AddDialogue` "Sparkles" "Have you found anything yet??" (select `bool` (`/Game/FirstPerson/Blueprints/BP_FirstPersonCharacter.FoundEye` _asbp_first_person_character_6) :`false` (`|MakeArray` "Not yet but Im still hopeful!" :!type "Text") :`true` (`|MakeArray` "" "Yes! Here it is!! The janitor even said they would vouch for you!" :!type "Text"))))
          (switch `/Game/Blueprint/Enum_DiaState` _state_19
            (:`NewEnumerator0`
              (switch `int` _optionindex_19
                (:`0`
                  _)
                (:`1`
                  (bind (_state_20 _optionindex_20) (`self.AddDialogue` "Sparkles" "OMG Thank you! Now the police can verify my story"))
                  (switch `/Game/Blueprint/Enum_DiaState` _state_20
                    (:`NewEnumerator0`
                      (switch `int` _optionindex_20
                        (:`0`
                          _))))))
              (`self.CloseConversation`))))))))