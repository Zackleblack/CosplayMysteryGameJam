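; BP_SuperFan is an interactable Super Fan character that the first-person player can talk to.
; The construction script writes CharacterName into a text label, which SetInteractableState shows or hides.
; On Interact, it stores the instigator, copies the dialogue tree index from the player's base dialogue component into its own dialogue component, and opens the conversation.
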(event `/Game/Blueprint/BPI_Interact.SetInteractableState`
  (params (bCanShowInteract :type Boolean))
  (if bCanShowInteract
    (`SceneComponent.SetVisibility` (`self.Txt_ChName`) true false)
    (else
      (`SceneComponent.SetVisibility` (`self.Txt_ChName`) false false))))

(event `/Game/Blueprint/BPI_Interact.Interact`
  (params (Instigator :type "Actor Object Reference"))
  (bind _output_get (set `self.Intergator` Instigator))
  (bind _asbp_first_person_character (cast `/Game/FirstPerson/Blueprints/BP_FirstPersonCharacter` _output_get))
  (set `/Game/Blueprint/AC_Dialogue_Base.DialogueTreeIndex` (`/Game/Blueprint/AC_Dialogue_Base.DialogueTreeIndex` (`/Game/FirstPerson/Blueprints/BP_FirstPersonCharacter.AC_Dialogue_Base` _asbp_first_person_character)) (`self.AC_DIalogueSuperFan`))
  (`/Game/Blueprint/AC_Dialogue_Base.OpenConversation` (`self.AC_DIalogueSuperFan`)))

(fn `UserConstructionScript`
  (`TextRenderComponent.K2_SetText` (`self.Txt_ChName`) (`self.CharacterName`)))