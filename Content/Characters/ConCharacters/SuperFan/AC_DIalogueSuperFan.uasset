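; Dialogue component for Phann, the superfan suspect in a convention murder mystery, who shares alibi details, clues and shipping opinions.
; Overrides Dialogue to pick a tree by DialogueTreeIndex for four time slots across two days, chaining AddDialogue option branches into CloseConversation.
; Player-character flags vary greetings and options for clues and the keychain side task.
; Some lines set flags on their Updated output, so insulting or enraging Phann sours later conversations.
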(fn `Dialogue`
  (bind _returnvalue (`GameplayStatics.GetPlayerPawn` 0))
  (bind _array (`|MakeArray` "Checking in, have you seen anything of note?" :!type "Text"))
  (bind _array_2 (`|MakeArray` "Continue" :!type "Text"))
  (`parent.Dialogue`)
  (set `self.DialogueIndex` -1)
  (switch `int` (`self.DialogueTreeIndex`)
    (:`0`
      ; Day 1 Afternoon
      (bind (_state _optionindex) (`self.AddDialogue` "Phann" "Crazy start to a con don't you think?" (`|MakeArray` "Where were you last night?" :!type "Text")))
      (switch `/Game/Blueprint/Enum_DiaState` _state
        (:`NewEnumerator0`
          (switch `int` _optionindex
            (:`0`
              (bind (_state_2 _optionindex_2) (`self.AddDialogue` "Phann" " I was at the back of the hall re-organising my Ita bag! I got lots of Kawaii~ merch of my OTP and NEEDED to put it in right away!" (`|MakeArray` "Did anyone see you doing this?" "What ship did you get merch of?" :!type "Text")))
              (switch `/Game/Blueprint/Enum_DiaState` _state_2
                (:`NewEnumerator0`
                  (switch `int` _optionindex_2
                    (:`0`
                      (bind (_state_3 _optionindex_3) (`self.AddDialogue` "Phann" "Yes! I was towards the door at the back off the hall where some of the staff was. I dropped some of my keychains and they were kind enough to help me pick them up!" (`|MakeArray` "Did you notice anything while over there?" "Did you find all of your keychains?" :!type "Text")))
                      (switch `/Game/Blueprint/Enum_DiaState` _state_3
                        (:`NewEnumerator0`
                          (switch `int` _optionindex_3
                            (:`0`
                              (bind (_state_4 _optionindex_4) (`self.AddDialogue` "Phann" "There was some lady yelling with the staff who wasn't helping me. Besides that I didn't see a lot." (`|MakeArray` "Continue" :!type "Text")))
                              (switch `/Game/Blueprint/Enum_DiaState` _state_4
                                (:`NewEnumerator0`
                                  (switch `int` _optionindex_4
                                    (:`0`
                                      (`self.CloseConversation` :!label _label))))
                                (:`NewEnumerator1`
                                  (bind _asbp_first_person_character (cast `/Game/FirstPerson/Blueprints/BP_FirstPersonCharacter` (`GameplayStatics.GetPlayerPawn` 0)))
                                  (set `/Game/FirstPerson/Blueprints/BP_FirstPersonCharacter.SpokeFan` true _asbp_first_person_character))))
                            (:`1`
                              (bind (_state_5 _optionindex_5) (`self.AddDialogue` "Phann" "Ugh I didnt! Wait, that could be good though right? If you find my  \nmissing keychain AND the staff guy remembers me that would  \nprove I’m innocent! Can you pweeeese go do that for me~?" (`|MakeArray` "Continue" :!type "Text")))
                              (switch `/Game/Blueprint/Enum_DiaState` _state_5
                                (:`NewEnumerator0`
                                  (switch `int` _optionindex_5
                                    (:`0`
                                      (goto _label))))))))))
                    (:`1`
                      (bind (_state_6 _optionindex_6) (`self.AddDialogue` "Phann" "Only the most perfect pair of all!!! John and James were meant for each other and no one can tell me otherwise!" (`|MakeArray` "I think John and Jamie actually belong together." "Absolutely! John and James are meant to be." :!type "Text")))
                      (switch `/Game/Blueprint/Enum_DiaState` _state_6
                        (:`NewEnumerator0`
                          (switch `int` _optionindex_6
                            (:`0`
                              (bind (_state_7 _optionindex_7) (`self.AddDialogue` "Phann" " …yeah I’m done talking with you" (`|MakeArray` "Continue" :!type "Text")))
                              (switch `/Game/Blueprint/Enum_DiaState` _state_7
                                (:`NewEnumerator0`
                                  (switch `int` _optionindex_7
                                    (:`0`
                                      (goto _label))))
                                (:`NewEnumerator1`
                                  (bind _asbp_first_person_character_2 (cast `/Game/FirstPerson/Blueprints/BP_FirstPersonCharacter` (`GameplayStatics.GetPlayerPawn` 0)))
                                  (set `/Game/FirstPerson/Blueprints/BP_FirstPersonCharacter.FanInsult` true _asbp_first_person_character_2))))
                            (:`1`
                              (bind (_state_8 _optionindex_8) (`self.AddDialogue` "Phann" "THANK YOU! That ship is so sugoi~! You know, I wasn't going to say anything about this, but since you're a fellow JoJa shipper I can trust you. I saw Reedee suspiciously running away from a vendor booth before Yo-yo was killed! It may be worth looking into. \n" (`|MakeArray` "Continue" :!type "Text")))
                              (switch `/Game/Blueprint/Enum_DiaState` _state_8
                                (:`NewEnumerator0`
                                  (switch `int` _optionindex_8
                                    (:`0`
                                      (goto _label))))))))))))))))))
    (:`1`
      (bind _asbp_first_person_character_3 (cast `/Game/FirstPerson/Blueprints/BP_FirstPersonCharacter` (`GameplayStatics.GetPlayerPawn` 0)))
      (if (`/Game/FirstPerson/Blueprints/BP_FirstPersonCharacter.FanInsult` _asbp_first_person_character_3)
        ;[0.15 0.04092 0.1024 0.5] 1Evening
        (bind (_state_9 _optionindex_9) (`self.AddDialogue` "Phann" "Looks like this absolute baka is back" _array))
        (switch `/Game/Blueprint/Enum_DiaState` _state_9
          (:`NewEnumerator0`
            (switch `int` _optionindex_9
              (:`0`
                _))))
        (else
          (bind (_state_10 _optionindex_10) (`self.AddDialogue` "Phann" "Omg Heyyyyyyy!" _array))
          (switch `/Game/Blueprint/Enum_DiaState` _state_10
            (:`NewEnumerator0`
              (switch `int` _optionindex_10
                (:`0`
                  _))))))
      (bind _asbp_first_person_character_4 (cast `/Game/FirstPerson/Blueprints/BP_FirstPersonCharacter` _returnvalue))
      (if (`/Game/FirstPerson/Blueprints/BP_FirstPersonCharacter.Second1A` _asbp_first_person_character_4)
        (bind _asbp_first_person_character_5 (cast `/Game/FirstPerson/Blueprints/BP_FirstPersonCharacter` _returnvalue))
        (bind (_state_11 _optionindex_11) (`self.AddDialogue` "Phann" "R: Nothing so far! But there's someone here now standing with his mom. It may be worth talking to him if you haven't already." (select `bool` (`/Game/FirstPerson/Blueprints/BP_FirstPersonCharacter.FoundKey` _asbp_first_person_character_5) :`false` (`|MakeArray` "What did you talk about Yo-Yo mon about?" :!type "Text") :`true` (`|MakeArray` "What did you talk about Yo-Yo mon about?" "I found your keychain!" :!type "Text"))))
        (switch `/Game/Blueprint/Enum_DiaState` _state_11
          (:`NewEnumerator0`
            (switch `int` _optionindex_11
              (:`0`
                (bind (_state_12 _optionindex_12) (`self.AddDialogue` "Phann" "Nothing sus I swear! Just talking about ships and my OTP. She and that other girl used to cosplay one of them and I wanted to know if they were planning to cosplay them again soon. Unfortunately Yo-Yo mon seemed VERY against that question. Bummers :(" (`|MakeArray` "What was Sparkles reaction?" :!type "Text")))
                (switch `/Game/Blueprint/Enum_DiaState` _state_12
                  (:`NewEnumerator0`
                    (switch `int` _optionindex_12
                      (:`0`
                        (bind (_state_13 _optionindex_13) (`self.AddDialogue` "Phann" "They didn't have much of any reaction. They seemed super bored since no one was in their line and Yo-Yo Mon was super busy with people." (`|MakeArray` "Thanks for your help!" :!type "Text")))
                        (switch `/Game/Blueprint/Enum_DiaState` _state_13
                          (:`NewEnumerator0`
                            (switch `int` _optionindex_13
                              (:`0`
                                _)))))))))
              (:`1`
                (bind (_state_14 _optionindex_14) (`self.AddDialogue` "Phann" "OMG YAY! This totally clears me right? I would love to stop worrying about this so I can focus on more important things like my ships." (`|MakeArray` "Glad I could help!" :!type "Text") :!label _label_2))
                (switch `/Game/Blueprint/Enum_DiaState` _state_14
                  (:`NewEnumerator0`
                    (switch `int` _optionindex_14
                      (:`0`
                        _))))))))
        (else
          (bind _asbp_first_person_character_6 (cast `/Game/FirstPerson/Blueprints/BP_FirstPersonCharacter` _returnvalue))
          (bind (_state_15 _optionindex_15) (`self.AddDialogue` "Phann" "R: Nothing so far! But there's someone here now standing with his mom. It may be worth talking to him if you haven't already." (select `bool` (`/Game/FirstPerson/Blueprints/BP_FirstPersonCharacter.FoundKey` _asbp_first_person_character_6) :`false` (`|MakeArray` "Thanks for your help!" :!type "Text") :`true` (`|MakeArray` "Thanks for your help!" "I found your keychain" :!type "Text"))))
          (switch `/Game/Blueprint/Enum_DiaState` _state_15
            (:`NewEnumerator0`
              (switch `int` _optionindex_15
                (:`0`
                  _)
                (:`1`
                  (goto _label_2)))))))
      (`self.CloseConversation`))
    (:`2`
      (bind _asbp_first_person_character_7 (cast `/Game/FirstPerson/Blueprints/BP_FirstPersonCharacter` (`GameplayStatics.GetPlayerPawn` 0)))
      ;[0.0413 0.05643 0.15 0.5] 2Morning
      (bind (_state_16 _optionindex_16) (`self.AddDialogue` "Phann" "Ohayo gozaimasu!!!~<3" (select `bool` (`/Game/FirstPerson/Blueprints/BP_FirstPersonCharacter.SpokeMom` _asbp_first_person_character_7) :`false` (`|MakeArray` "Did the kid you mentioned before previously have a phone?" "Where is Redee?" :!type "Text") :`true` (`|MakeArray` "Did the kid you mentioned before previously have a phone?" "Where is Redee?" "Why are you so chipper today?" :!type "Text"))))
      (switch `/Game/Blueprint/Enum_DiaState` _state_16
        (:`NewEnumerator0`
          (switch `int` _optionindex_16
            (:`0`
              (bind (_state_17 _optionindex_17) (`self.AddDialogue` "Phann" "OH HE TOTALLY DID! It was on a long selfie stick and he was like, constantly filming on it. You know, I bet there's totally some evidence to clear someone on there! Hopefully me since I should be pretty easy to spot in a crowd." _array_2))
              (switch `/Game/Blueprint/Enum_DiaState` _state_17
                (:`NewEnumerator0`
                  (switch `int` _optionindex_17
                    (:`0`
                      (`self.CloseConversation` :!label _label_3))))))
            (:`1`
              (bind (_state_18 _optionindex_18) (`self.AddDialogue` "Phann" "I thought it smelled better in here today! I have no clue where he went, all I can say is sayonara to that stink." _array_2))
              (switch `/Game/Blueprint/Enum_DiaState` _state_18
                (:`NewEnumerator0`
                  (switch `int` _optionindex_18
                    (:`0`
                      (goto _label_3))))))
            (:`2`
              (bind (_state_19 _optionindex_19) (`self.AddDialogue` "Phann" "I had an awesome idea for a fanfic last night based off what happened IRL! What if John and Jamie went on a date to a convention, BUT Jamie died at the con just like what happened! Then John and James could meet there, fall hopelessly in love, and my OTP could have the happy ending they deserve." (`|MakeArray` "Why would you write something like that???" "Ah, interesting.." :!type "Text")))
              (switch `/Game/Blueprint/Enum_DiaState` _state_19
                (:`NewEnumerator0`
                  (switch `int` _optionindex_19
                    (:`0`
                      (bind (_state_20 _optionindex_20) (`self.AddDialogue` "Phann" "It's called art. Obviously. You clearly need to pick up a manga or open AO3 and experience actual culture."))
                      (switch `/Game/Blueprint/Enum_DiaState` _state_20
                        (:`NewEnumerator0`
                          (switch `int` _optionindex_20
                            (:`0`
                              (goto _label_3))))
                        (:`NewEnumerator1`
                          (bind _asbp_first_person_character_8 (cast `/Game/FirstPerson/Blueprints/BP_FirstPersonCharacter` (`GameplayStatics.GetPlayerPawn` 0)))
                          (set `/Game/FirstPerson/Blueprints/BP_FirstPersonCharacter.FanEnrage` true _asbp_first_person_character_8))))
                    (:`1`
                      (goto _label_3))))))))))
    (:`3`
      (bind _asbp_first_person_character_9 (cast `/Game/FirstPerson/Blueprints/BP_FirstPersonCharacter` (`GameplayStatics.GetPlayerPawn` 0)))
      (if (`/Game/FirstPerson/Blueprints/BP_FirstPersonCharacter.FanEnrage` _asbp_first_person_character_9)
        ;[0.15 0.4203 0.15 0.5] 2Afternoon
        (bind (_state_21 _optionindex_21) (`self.AddDialogue` "Phann" "Ew, get away from me fake fan" (`|MakeArray` "Continue" :!type "Text")))
        (switch `/Game/Blueprint/Enum_DiaState` _state_21
          (:`NewEnumerator0`
            (switch `int` _optionindex_21
              (:`0`
                _))))
        (else
          (bind (_state_22 _optionindex_22) (`self.AddDialogue` "Phann" "Ohayo gozaimasu!!!~<3" (`|MakeArray` "Seen anything else?" :!type "Text")))
          (switch `/Game/Blueprint/Enum_DiaState` _state_22
            (:`NewEnumerator0`
              (switch `int` _optionindex_22
                (:`0`
                  (bind (_state_23 _optionindex_23) (`self.AddDialogue` "Phann" "That weird guy is back and he somehow looks and smells worse. I’d talk to him myself but I don't want to be near…that. Plus the kid is near him and is waving around that selfie stick again and I don't trust him to not hit me or someone else." (`|MakeArray` "Thanks for the tip!" :!type "Text")))
                  (switch `/Game/Blueprint/Enum_DiaState` _state_23
                    (:`NewEnumerator0`
                      (switch `int` _optionindex_23
                        (:`0`
                          _))))))))))
      (`self.CloseConversation`))))

(fn `NewFunction_0`)