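; Base dialogue component that opens and closes a conversation widget and leaves the Dialogue function empty, apparently for child classes to script.
; ProgressDialogue resets the step index and replays Dialogue from the start.
; Each AddDialogue call returns the option stored for that step in the DialogueProgress map, or sends the line to the widget if none exists.
; Helpers record choices, roll back or clear progress, and adjust tree indices.
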(fn `AddDialogue`
  (params (Speaker :type Text) (Dialogue :type Text) (Options :type "Array of Text"))
  (returns (State :type "/Game/Blueprint/Enum_DiaState Enum") (OptionIndex :type Integer))
  (bind (_value _returnvalue) (`BlueprintMapLibrary.Map_Find` (`self.DialogueProgress`) (`self.DialogueIndex`)))
  (`/Engine/EditorBlueprintResources/StandardMacros.IncrementInt` (`self.DialogueIndex`)
    (:`  `
      (if _returnvalue
        (return "NewEnumerator0" _value)
        (else
          (`/Game/Widgets/W_Dialogue.UpdateDialogue` (`self.DialogueWidget`) (`self.DialogueIndex`) (`local.Speaker`) (`local.Dialogue`) (`local.Options`))
          (return "NewEnumerator1" 0))))))

(fn `AddDialogueTreeIndex`
  (set `self.DialogueTreeIndex` (+ (`self.DialogueTreeIndex`) 1)))

(fn `ClearDialogueProgress`
  (`BlueprintMapLibrary.Map_Clear` (`self.DialogueProgress`)))

(fn `CloseConversation`
  (bind _returnvalue (`GameplayStatics.GetPlayerController` 0))
  (`Widget.RemoveFromParent` (`self.DialogueWidget`))
  (`WidgetBlueprintLibrary.SetInputMode_GameOnly` _returnvalue)
  (set `PlayerController.bShowMouseCursor` false _returnvalue)
  (`BlueprintMapLibrary.Map_Clear` (`self.DialogueProgress`)))

(fn `Dialogue`)

(fn `OpenConversation`
  (bind _returnvalue (`|CreateWidget` "/Game/Widgets/W_Dialogue.W_Dialogue_C" null self))
  (bind _output_get (set `self.DialogueWidget` _returnvalue))
  (`UserWidget.AddToViewport` _output_get 0)
  (`self.ProgressDialogue`))

(fn `ProgressDialogue`
  (set `self.DialogueIndex` -1)
  (`self.Dialogue`))

(fn `RemoveDialogueProgress`
  (params (ProgressStep :type Integer))
  (for _index (range (+ ProgressStep 1))
    (`BlueprintMapLibrary.Map_Remove` (`self.DialogueProgress`) (- (`self.DialogueIndex`) _index))))

(fn `SetDialogueTreeIndex`
  (params (DialogueTreeIndex :type Integer))
  (set `self.DialogueIndex` DialogueTreeIndex)
  (`self.ClearDialogueProgress`))

(fn `UpdateSelectedOption`
  (params (ProgressIndex :type "Integer (by ref)") (OptionIndex :type "Integer (by ref)"))
  (`BlueprintMapLibrary.Map_Add` (`self.DialogueProgress`) ProgressIndex OptionIndex))