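; Dialogue component for the SuperFan character, defining a short branching conversation about cheese.
; The Dialogue override calls its parent, resets DialogueIndex, then switches on DialogueTreeIndex, with only the first tree defined.
; Each AddDialogue node supplies speaker, line and options, and its Pass Through state branches on the chosen option.
; The follow-up lines end without further branches, and NewFunction is an empty stub.
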(fn `Dialogue`
  (`parent.Dialogue`)
  (set `self.DialogueIndex` -1)
  (switch `int` (`self.DialogueTreeIndex`)
    (:`0`
      (bind (_state _optionindex) (`self.AddDialogue` "SuperFan" "Hi, do you have cheese" (`|MakeArray` "Yes" "No" :!type "Text")))
      (switch `/Game/Blueprint/Enum_DiaState` _state
        (:`NewEnumerator0`
          (switch `int` _optionindex
            (:`0`
              (bind (_state_2 _optionindex_2) (`self.AddDialogue` "SuperFan" "Cool! Can I have some??" (`|MakeArray` "Yes" "No" :!type "Text")))
              (switch `/Game/Blueprint/Enum_DiaState` _state_2
                (:`NewEnumerator0`
                  (switch `int` _optionindex_2))))
            (:`1`
              (bind (_state_3 _optionindex_3) (`self.AddDialogue` "SuperFan" "Aww rats" (`|MakeArray` "Continue" :!type "Text")))
              (switch `/Game/Blueprint/Enum_DiaState` _state_3
                (:`NewEnumerator0`
                  (switch `int` _optionindex_3))))))))))

(fn `NewFunction`)